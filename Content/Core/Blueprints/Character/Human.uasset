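; Human player character Blueprint for an action RPG, handling movement, camera, jump, crouch, sprint, attack and dodge input.
; Input events drive movement and set pressed/released flags in an input buffer, with a timer splitting the Sprint key into hold-to-sprint and tap-to-dodge.
; Each Tick, the Anim macro polls the buffer while grounded with no full-body montage playing, choosing an attack montage or a directional roll relative to control yaw.
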(event Custom|InvokeSprint
  (Class|CharacterBase|InvokeChangeMoveGait "Sprinting"))

(event EventBeginPlay)

(event Collision|EventActorBeginOverlap
  (params (OtherActor :type Actor%20Object%20Reference)))

(event EventTick
  (params (DeltaSeconds :type Float%20%28single-precision%29))
  (|Anim))

(event Input|ActionEvents|InputActionSprint
  (params (Key :type Key%20Structure))
  (:Pressed
    (bind _returnvalue (Utilities|Time|SetTimerbyEvent (delegate Custom|InvokeSprint) 0.2)))
  (:Released
    (if (Utilities|Time|IsTimerActivebyHandle _returnvalue)
      (Utilities|Time|ClearandInvalidateTimerbyHandle _returnvalue)
      (Utilities|SetInputBuffer "Dodge" :!label _label
        (:Pressed_
          (Utilities|FlowControl|Delay 0.2)
          (goto _label Released)))
      (else
        (Class|CharacterBase|InvokeChangeMoveGait "Running")))))

(event Input|ActionEvents|InputActionCrouch
  (params (Key :type Key%20Structure))
  (:Pressed
    (Utilities|SetInputBuffer "Down" :!label _label
      (:Pressed_
        (Character|Crouch))
      (:Released_
        (Character|UnCrouch))))
  (:Released
    (goto _label Released)))

(event Input|ActionEvents|InputActionLeftLightAttack
  (params (Key :type Key%20Structure))
  (:Pressed
    (Utilities|SetInputBuffer "LeftLightAttack" :!label _label))
  (:Released
    (goto _label Released)))

(event Input|ActionEvents|InputActionLeftHeavyAttack
  (params (Key :type Key%20Structure))
  (:Pressed
    (Utilities|SetInputBuffer "LeftHeavyAttack" :!label _label))
  (:Released
    (goto _label Released)))

(event Input|ActionEvents|InputActionRightLightAttack
  (params (Key :type Key%20Structure))
  (:Pressed
    (Utilities|SetInputBuffer "RightLightAttack" :!label _label))
  (:Released
    (goto _label Released)))

(event Input|ActionEvents|InputActionRightHeavyAttack
  (params (Key :type Key%20Structure))
  (:Pressed
    (Utilities|SetInputBuffer "RightHeavyAttack" :!label _label))
  (:Released
    (goto _label Released)))

(event Input|ActionEvents|InputActionJump
  (params (Key :type Key%20Structure))
  (:Pressed
    (Utilities|SetInputBuffer "Up" :!label _label
      (:Pressed_
        (Character|Jump))
      (:Released_
        (Character|StopJumping))))
  (:Released
    (goto _label Released)))

(event Input|AxisEvents|InputAxisLookUp
  (params (AxisValue :type Float%20%28single-precision%29))
  (Pawn|Input|AddControllerPitchInput AxisValue))

(event Input|AxisEvents|InputAxisTurn
  (params (AxisValue :type Float%20%28single-precision%29))
  (Pawn|Input|AddControllerYawInput AxisValue))

(event Input|AxisEvents|InputAxisMoveForward
  (params (AxisValue :type Float%20%28single-precision%29))
  (Pawn|Input|AddMovementInput (Math|Vector|GetForwardVector (Math|Rotator|MakeRotator 0.0 0.0 (.Yaw (Math|Rotator|BreakRotator (Pawn|GetControlRotation :!class /Script/Engine.Pawn))))) AxisValue false)
  (Utilities|SetInputBufferbyValue "Forward" "Backward" AxisValue))

(event Input|AxisEvents|InputAxisMoveRight
  (params (AxisValue :type Float%20%28single-precision%29))
  (Pawn|Input|AddMovementInput (Math|Vector|GetRightVector (Math|Rotator|MakeRotator 0.0 0.0 (.Yaw (Math|Rotator|BreakRotator (Pawn|GetControlRotation :!class /Script/Engine.Pawn))))) AxisValue false)
  (Utilities|SetInputBufferbyValue "Right" "Left" AxisValue))

(fn ConstructionScript)

(fn DodogebyDirection
  (params (YawOffset :type Float%20%28single-precision%29))
  (bind _returnvalue (Transformation|GetActorRotation))
  (bind _returnvalue_2 (Pawn|GetControlRotation :!class /Script/Engine.Pawn))
  (bind _returnvalue_3 (+ (.yaw _returnvalue_2) YawOffset))
  (bind _returnvalue_4 (Math|Rotator|Delta(Rotator) _returnvalue (Math|Rotator|MakeRotator (.roll _returnvalue_2) (.pitch _returnvalue_2) _returnvalue_3)))
  (if (Math|Float|InRange(Float) (.yaw _returnvalue_4) -45.0 45.0)
    (Class|CharacterBase|PlayMontage "/Game/Assets/Character/Human/Anims/Battle/H_Rolling_Front_Montage.H_Rolling_Front_Montage" 1.0 "None" true)
    (elif (Math|Float|InRange(Float) (.yaw _returnvalue_4) -135.0 -45.0 true false)
      (Class|CharacterBase|PlayMontage "/Game/Assets/Character/Human/Anims/Battle/H_Rolling_Right_Montage.H_Rolling_Right_Montage" 1.0 "None" true)
      (elif (Math|Float|InRange(Float) (.yaw _returnvalue_4) 45.0 135.0 false)
        (Class|CharacterBase|PlayMontage "/Game/Assets/Character/Human/Anims/Battle/H_Rolling_Left_Montage.H_Rolling_Left_Montage" 1.0 "None" true)
        (else
          (Class|CharacterBase|PlayMontage "/Game/Assets/Character/Human/Anims/Battle/H_Rolling_Back_Montage.H_Rolling_Back_Montage" 1.0 "None" true))))))